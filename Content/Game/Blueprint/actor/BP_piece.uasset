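; BP_piece is a coin pickup actor that the player character collects by walking into it.
; A timeline started on BeginPlay animates the Cylinder mesh's relative location while it still exists.
; Box overlap with BP_ThirdPersonCharacter disables actor collision, calls Addcoin on BP_ThirdPersonGameMode and destroys the Cylinder component, leaving the actor itself in place.
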(event `self.ReceiveBeginPlay`
  (bind _cylinder (`self.Cylinder`))
  (bind (_direction _newtrack_0) (`Timeline|Timeline`)
    (:`Update`
      (`/Engine/EditorBlueprintResources/StandardMacros.IsValid` _cylinder
        (:`Is Valid`
          (`SceneComponent.K2_SetRelativeLocation` _cylinder _newtrack_0 false false))))))

(event `self.Box.OnComponentBeginOverlap`
  (params (OverlappedComponent :type "PrimitiveComponent Object Reference") (OtherActor :type "Actor Object Reference") (OtherComp :type "PrimitiveComponent Object Reference") (OtherBodyIndex :type Integer) (bFromSweep :type Boolean) (SweepResult :type "HitResult Structure (by ref)"))
  (cast `/Game/ThirdPerson/Blueprints/BP_ThirdPersonCharacter` OtherActor)
  (`self.SetActorEnableCollision` false)
  (bind _asbp_third_person_game_mode (cast `/Game/ThirdPerson/Blueprints/BP_ThirdPersonGameMode` (`GameplayStatics.GetGameMode`)))
  (`/Game/ThirdPerson/Blueprints/BP_ThirdPersonGameMode.addcoin` _asbp_third_person_game_mode)
  (`ActorComponent.K2_DestroyComponent` (`self.Cylinder`)))

(fn `UserConstructionScript`)