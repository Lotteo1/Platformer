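; Spike trap actor that moves its mesh vertically and costs the third-person player a life on contact.
; After a configurable StartDelay from BeginPlay, a timeline drives the static mesh's relative Z position.
; When a box component overlaps BP_ThirdPersonCharacter, it calls LoseLife and Respawn on BP_ThirdPersonGameMode.
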(event `self.ReceiveBeginPlay`
  (`KismetSystemLibrary.Delay` (`self.start delay`))
  (bind (_direction _hight) (`Timeline|Timeline`)
    (:`Update`
      (`SceneComponent.K2_SetRelativeLocation` (`self.StaticMesh`) (`KismetMathLibrary.MakeVector` 0.0 0.0 _hight) false false))))

(event `self.Box.OnComponentBeginOverlap`
  (params (OverlappedComponent :type "PrimitiveComponent Object Reference") (OtherActor :type "Actor Object Reference") (OtherComp :type "PrimitiveComponent Object Reference") (OtherBodyIndex :type Integer) (bFromSweep :type Boolean) (SweepResult :type "HitResult Structure (by ref)"))
  (cast `/Game/ThirdPerson/Blueprints/BP_ThirdPersonCharacter` OtherActor)
  (bind _asbp_third_person_game_mode (cast `/Game/ThirdPerson/Blueprints/BP_ThirdPersonGameMode` (`GameplayStatics.GetGameMode`)))
  (`/Game/ThirdPerson/Blueprints/BP_ThirdPersonGameMode.lose life` _asbp_third_person_game_mode)
  (`/Game/ThirdPerson/Blueprints/BP_ThirdPersonGameMode.respawn` _asbp_third_person_game_mode))

(fn `UserConstructionScript`)